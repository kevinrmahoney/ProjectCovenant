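; First-person character controller Blueprint that handles walking, sprinting, mouse look and automatic shooting.
; Movement follows control yaw, and Sprint switches the walk speed between run and sprint values.
; Holding Shoot runs a Gate loop that spawns a BasicBullet at BulletSpawn, pushes it along the camera's forward vector with a physics impulse and plays a gunshot.
; A CanShoot flag and Delay set the fire rate until release closes the gate.
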(event Collision|EventActorBeginOverlap
  (params (OtherActor :type Actor%20Object%20Reference)))

(event Input|ActionEvents|InputActionJump
  (params (Key :type Key%20Structure :default "AnyKey"))
  ;[1 1 1] Movement
)

(event Input|ActionEvents|InputActionShoot
  (params (Key :type Key%20Structure :default "AnyKey"))
  ;[1 1 1] Shooting
  (:Pressed
    (Utilities|FlowControl|Sequence
      (:then_0
        (goto _label Open))
      (:then_1
        (Utilities|FlowControl|Gate true :!label _label
          (:Exit
            (Utilities|FlowControl|Sequence
              (:then_0
                (if (Variables|Default|GetCanShoot)
                  (Utilities|FlowControl|Sequence
                    (:then_0
                      (bind _returnvalue (Game|SpawnActorfromClass "/Game/Blueprints/BasicBullet.BasicBullet_C" (Transformation|GetWorldTransform (Variables|Default|GetBulletSpawn)) "Undefined" 0 0))
                      (Physics|AddImpulse (Variables|/Game/Blueprints/BasicBullet.BasicBullet_C|GetCylinder _returnvalue) (* (Math|Vector|GetForwardVector (Transformation|GetWorldRotation (Variables|Default|GetCamera))) (Variables|Default|GetBulletSpeed)) "None" false))
                    (:then_1
                      (Class|FMODAudioComponent|Play (Variables|Default|GetGunshot))))))
              (:then_1
                (Variables|Default|SetCanShoot false)
                (Utilities|FlowControl|Delay (Variables|Default|GetShootingRate))
                (Variables|Default|SetCanShoot true)
                (goto _label))))))))
  (:Released
    (goto _label Close)))

(event Input|ActionEvents|InputActionSprint
  (params (Key :type Key%20Structure :default "AnyKey"))
  (bind _charactermovement (Variables|Character|GetCharacterMovement))
  ;[1 1 1] Movement
  (:Pressed
    (Variables|/Script/Engine.CharacterMovementComponent|SetMaxWalkSpeed _charactermovement (Variables|Default|GetSprintSpeed)))
  (:Released
    (Variables|/Script/Engine.CharacterMovementComponent|SetMaxWalkSpeed _charactermovement (Variables|Default|GetRunSpeed))))

(event Input|AxisEvents|InputAxisMouseLookHorizontal
  (params (AxisValue :type Float%20%28single-precision%29))
  ;[1 1 1] Mouse Look
  (Pawn|Input|AddControllerYawInput AxisValue))

(event Input|AxisEvents|InputAxisMouseLookVertical
  (params (AxisValue :type Float%20%28single-precision%29))
  ;[1 1 1] Mouse Look
  (Pawn|Input|AddControllerPitchInput AxisValue))

(event Input|AxisEvents|InputAxisHorizontal
  (params (AxisValue :type Float%20%28single-precision%29))
  ;[1 1 1] Movement
  (Pawn|Input|AddMovementInput (Math|Vector|GetRightVector (Math|Rotator|MakeRotator 0.0 0.0 (.yaw (Pawn|GetControlRotation :!class /Script/Engine.Pawn)))) AxisValue false))

(event Input|AxisEvents|InputAxisVertical
  (params (AxisValue :type Float%20%28single-precision%29))
  ;[1 1 1] Movement
  (Pawn|Input|AddMovementInput (Math|Vector|GetForwardVector (Math|Rotator|MakeRotator 0.0 0.0 (.yaw (Pawn|GetControlRotation :!class /Script/Engine.Pawn)))) AxisValue false))

(fn ConstructionScript)
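; Target actor with outer, middle and inner rings that flashes a light for whichever ring gets hit.
; Each ring's OnComponentHit raises the intensity of its matching hit light.
; All three events feed one shared half-second Delay, then TurnOffAll zeroes every light, so hits during a running delay do not extend the flash.
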(event OnComponentHit(OutsideRing)
  (params (HitComponent :type Primitive%20Component%20Object%20Reference) (OtherActor :type Actor%20Object%20Reference) (OtherComp :type Primitive%20Component%20Object%20Reference) (NormalImpulse :type Vector :default "0, 0, 0") (Hit :type Hit%20Result%20Structure%20%28by%20ref%29))
  (CallFunction|TurnonOuter)
  (Utilities|FlowControl|Delay 0.5)
  (CallFunction|TurnOffAll))

(event OnComponentHit(MiddleRing)
  (params (HitComponent :type Primitive%20Component%20Object%20Reference) (OtherActor :type Actor%20Object%20Reference) (OtherComp :type Primitive%20Component%20Object%20Reference) (NormalImpulse :type Vector :default "0, 0, 0") (Hit :type Hit%20Result%20Structure%20%28by%20ref%29))
  (CallFunction|TurnonMiddle)
  (Utilities|FlowControl|Delay 0.5)
  (CallFunction|TurnOffAll))

(event OnComponentHit(InnerRing)
  (params (HitComponent :type Primitive%20Component%20Object%20Reference) (OtherActor :type Actor%20Object%20Reference) (OtherComp :type Primitive%20Component%20Object%20Reference) (NormalImpulse :type Vector :default "0, 0, 0") (Hit :type Hit%20Result%20Structure%20%28by%20ref%29))
  (CallFunction|TurnonInner)
  (Utilities|FlowControl|Delay 0.5)
  (CallFunction|TurnOffAll))

(fn ConstructionScript)

(fn TurnOffAll
  (Utilities|FlowControl|Sequence
    (:then_0
      (Rendering|Components|Light|SetIntensity (Variables|Default|GetOuterRingHit) 0.0))
    (:then_1
      (Rendering|Components|Light|SetIntensity (Variables|Default|GetMiddleRingHit) 0.0))
    (:then_2
      (Rendering|Components|Light|SetIntensity (Variables|Default|GetInnerRingHit) 0.0))))

(fn TurnonInner
  (Rendering|Components|Light|SetIntensity (Variables|Default|GetInnerRingHit) 5e+03))

(fn TurnonMiddle
  (Rendering|Components|Light|SetIntensity (Variables|Default|GetMiddleRingHit) 5e+03))

(fn TurnonOuter
  (Rendering|Components|Light|SetIntensity (Variables|Default|GetOuterRingHit) 5e+03))